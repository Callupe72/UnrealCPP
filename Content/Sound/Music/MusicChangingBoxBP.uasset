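; A trigger box actor that switches the level's music track when the player pawn enters or leaves it.
; A WhenPlaySound mode selects switching on enter, on exit, or only while inside, where it saves the current track index and restores it on exit.
; It finds the first MusicManagerBP if none is set and calls ChangeMusicTo on it.
; The construction script labels the box with the track name, index and mode through a TextRender.
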(event `self.ReceiveBeginPlay`
  (`/Engine/EditorBlueprintResources/StandardMacros.IsValid` (`self.MusicManager`)
    (:`Is Not Valid`
      (bind _outactors (`GameplayStatics.GetAllActorsOfClass` "/Game/Sound/Music/MusicManagerBP.MusicManagerBP_C"))
      (set `self.MusicManager` (`|GetArrayItem` _outactors)))))

(event `self.Box.OnComponentBeginOverlap`
  (params (OverlappedComponent :type "PrimitiveComponent Object Reference") (OtherActor :type "Actor Object Reference") (OtherComp :type "PrimitiveComponent Object Reference") (OtherBodyIndex :type Integer) (bFromSweep :type Boolean) (SweepResult :type "HitResult Structure (by ref)"))
  (bind _musicmanager (`self.MusicManager`))
  (if (== OtherActor (`GameplayStatics.GetPlayerPawn` 0))
    (switch `/Game/Sound/Music/SoundActivation` (`self.WhenPlaySound`)
      (:`NewEnumerator0`
        _)
      (:`NewEnumerator2`
        (set `self.PreviousSoundIndex` (`/Game/Sound/Music/MusicManagerBP.CurrentSoundIndex` _musicmanager))))
    (`/Game/Sound/Music/MusicManagerBP.ChangeMusicTo` _musicmanager (`self.Song to Play Index`))))

(event `self.Box.OnComponentEndOverlap`
  (params (OverlappedComponent :type "PrimitiveComponent Object Reference") (OtherActor :type "Actor Object Reference") (OtherComp :type "PrimitiveComponent Object Reference") (OtherBodyIndex :type Integer))
  (if (== OtherActor (`GameplayStatics.GetPlayerPawn` 0))
    (switch `/Game/Sound/Music/SoundActivation` (`self.WhenPlaySound`)
      (:`NewEnumerator1`
        (`/Game/Sound/Music/MusicManagerBP.ChangeMusicTo` (`self.MusicManager`) (`self.Song to Play Index`)))
      (:`NewEnumerator2`
        (`/Game/Sound/Music/MusicManagerBP.ChangeMusicTo` (`self.MusicManager`) (`self.PreviousSoundIndex`))))))

(fn `ChangeTextDebug`
  (`TextRenderComponent.K2_SetText` (`self.TextRender`) (`KismetTextLibrary.Conv_StringToText` (`KismetStringLibrary.Concat_StrStr` "PLAY SOUND " (`KismetSystemLibrary.GetDisplayName` (`|GetArrayItem` (`/Game/Sound/Music/MusicManagerBP.TrackList` (`self.MusicManager`)) (`self.Song to Play Index`))) "(" (`KismetStringLibrary.Conv_IntToString` (`self.Song to Play Index`)) ") " (`|GetEnumeratorNameAsString` (`self.WhenPlaySound`))))))

(fn `UserConstructionScript`
  (`/Engine/EditorBlueprintResources/StandardMacros.IsValid` (`self.MusicManager`)
    (:`Is Valid`
      _)
    (:`Is Not Valid`
      (bind _outactors (`GameplayStatics.GetAllActorsOfClass` "/Game/Sound/Music/MusicManagerBP.MusicManagerBP_C"))
      (set `self.MusicManager` (`|GetArrayItem` _outactors))))
  (`self.ChangeTextDebug`))