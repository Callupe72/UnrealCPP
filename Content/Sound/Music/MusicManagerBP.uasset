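; Music manager Blueprint that plays a list of tracks and crossfades between them by index.
; On BeginPlay it starts every track as a muted 2D sound, then raises the starting song to MusicVolume.
; ChangeMusicTo runs a timeline that inversely blends the current and target track volumes, then updates the current reference and index.
; The crossfade works on a 0 to 1 curve without applying MusicVolume.
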(event `self.ReceiveBeginPlay`
  (bind _output (`|GetArrayItem` (`self.MusicRefs`) (`self.SongToPlay`)))
  (for _array_element (`self.TrackList`)
    (bind _returnvalue (`GameplayStatics.CreateSound2D` _array_element 1.0 1.0 0.0 null))
    (`KismetArrayLibrary.Array_Add` (`self.MusicRefs`) _returnvalue)
    (`AudioComponent.SetVolumeMultiplier` _returnvalue 0.0)
    (`AudioComponent.Play` _returnvalue 0.0))
  (`AudioComponent.SetVolumeMultiplier` _output (`self.MusicVolume`))
  (set `self.CurrentMusicRef` _output)
  (set `self.CurrentSoundIndex` (`self.SongToPlay`)))

(event `ChangeMusicTo`
  (params (SongToPlayIndex :type Integer))
  (bind _output (`|GetArrayItem` (`self.MusicRefs`) SongToPlayIndex))
  (bind (_direction _newtrack_0) (`Timeline|SoundTransition` :!via `PlayFromStart`)
    (:`Update`
      (`AudioComponent.SetVolumeMultiplier` (`self.CurrentMusicRef`) (- 1.0 _newtrack_0))
      (`AudioComponent.SetVolumeMultiplier` _output _newtrack_0))
    (:`Finished`
      (set `self.CurrentMusicRef` _output)
      (set `self.CurrentSoundIndex` SongToPlayIndex)
      (`KismetSystemLibrary.PrintString` (`KismetStringLibrary.Concat_StrStr` "I'm now playing sound " (`KismetStringLibrary.Conv_IntToString` SongToPlayIndex))))))

(fn `UserConstructionScript`)